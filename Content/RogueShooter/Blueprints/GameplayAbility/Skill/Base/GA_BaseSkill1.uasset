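; GA_BaseSkill1 is a hold-to-fire Gameplay Ability that shoots ice-impact projectiles from the avatar.
; On activation it spawns a BP_BaseProjectile just above the actor's location, aimed along the Character's control rotation, with fixed damage.
; It also starts a short looping timer through a Create Event delegate, presumably to repeat the shot.
; A WaitInputRelease task clears that timer and ends the ability when input is released.
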(event Ability|EventActivateAbility
  (Utilities|FlowControl|Sequence
    (:then_0
      (Ability|Tasks|WaitInputRelease false
        (:OnRelease
          (Utilities|Time|ClearandInvalidateTimerbyHandle (Variables|Default|GetTimerHandle))
          (Ability|EndAbility))))
    (:then_1
      (CallFunction|GABaseSkill1AutoGenFunc)
      (bind _returnvalue (Utilities|Time|SetTimerbyEvent (EventDispatchers|CreateEvent :!event GABaseSkill1AutoGenFunc) 0.3 true :!label _label))
      (Variables|Default|SetTimerHandle _returnvalue))
    (:then_2
      (goto _label))))

(event Ability|EventOnEndAbility
  (params (bWasCancelled :type Boolean)))

(fn GABaseSkill1AutoGenFunc
  (bind _returnvalue (Ability|GetAvatarActorfromActorInfo))
  (bind _ascharacter (Utilities|Casting|CastToCharacter _returnvalue))
  (Game|SpawnActorfromClass "/Game/RogueShooter/Blueprints/Abilities/BP_BaseProjectile.BP_BaseProjectile_C" (Math|Transform|MakeTransform (+ (Transformation|GetActorLocation _returnvalue) "0.000000,0.000000,50.000000") (Pawn|GetControlRotation _ascharacter :!class /Script/Engine.Pawn)) "Undefined" "MultiplyWithRoot" _returnvalue "/Game/SurvivorsTemplate/Demo/Effects/FX_Combat_Ice/Impact/P_Impact_Ice.P_Impact_Ice" 1e+01 0))